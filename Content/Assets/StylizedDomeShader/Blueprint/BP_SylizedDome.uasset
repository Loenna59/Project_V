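; BP_SylizedDome is a showcase actor for stylized dome materials, displayed on a Sphere mesh set in the construction script.
; A and D step backward or forward through the Material array with wraparound, and C toggles two cameras.
; Space starts an automated tour that orbits the spring arm while a self-retriggering CameraZoom event advances materials and alternates arm zoom via FlipFlop and timeline, without wrapping the index.
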(event Custom|UpdateMat
  (params (+%20/%20- :type Boolean))
  (bind _index (Variables|Default|GetIndex))
  (if +%20/%20-
    (Math|Integer|IncrementInt _index
      (:%20%20
        _))
    (else
      (Math|Integer|DecrementInt _index
        (:%20%20
          _))))
  (Rendering|Material|SetMaterial (Variables|Default|GetSphere) 0 (Utilities|Array|Get(acopy) (Variables|Default|GetMaterial) _index)))

(event Custom|CameraZoom
  (CallFunction|UpdateMat true)
  (Utilities|FlowControl|Delay 1.0)
  (Utilities|FlowControl|FlipFlop
    (:A
      (bind _newtrack_0 (Timeline|Timeline PlayFromStart)
        (:Update
          (Variables|/Script/Engine.SpringArmComponent|SetTargetArmLength (Variables|Default|GetSpringArm) (Math|Float|Lerp 9e+02 8.5e+02 _newtrack_0)))
        (:Finished
          (CallFunction|CameraZoom))))
    (:B
      (Timeline|Timeline ReverseFromEnd))))

(event Input|KeyboardEvents|C
  (params (Key :type Key%20Structure))
  (:Pressed
    (Components|Activation|ToggleActive (Variables|Default|GetCamera))))

(event Input|KeyboardEvents|D
  (params (Key :type Key%20Structure))
  (:Pressed
    (if (< (Variables|Default|GetIndex) 19)
      _
      (else
        (Variables|Default|SetIndex -1)))
    (CallFunction|UpdateMat true)))

(event Input|KeyboardEvents|A
  (params (Key :type Key%20Structure))
  (:Pressed
    (if (> (Variables|Default|GetIndex) 0)
      _
      (else
        (Variables|Default|SetIndex 20)))
    (CallFunction|UpdateMat false)))

(event Input|KeyboardEvents|SpaceBar
  (params (Key :type Key%20Structure))
  (:Pressed
    (Variables|Default|SetIndex -1)
    (CallFunction|CameraZoom)
    (Components|Timeline|SetPlayRate (Variables|Default|Getrotation_tl) 0.5)
    (bind _newtrack_0 (Timeline|rotation_tl PlayFromStart)
      (:Update
        (Transformation|SetRelativeRotation (Variables|Default|GetSpringArm) (Math|Rotator|MakeRotator 0.0 -27.0 (* _newtrack_0 -1.0)) false false)))))

(fn ConstructionScript
  (Rendering|Material|SetMaterial (Variables|Default|GetSphere) 0 (Utilities|Array|Get(acopy) (Variables|Default|GetMaterial) (Variables|Default|GetIndex)))
  (Components|StaticMesh|SetStaticMesh (Variables|Default|GetSphere) (Variables|Default|GetNew%20Mesh))
  (Variables|Default|SetActive%20Mat (Utilities|Array|Get(acopy) (Variables|Default|GetMaterial) (Variables|Default|GetIndex))))