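; BP_RadarEffect is a boss-related Blueprint for a radar visual effect built on a Sphere mesh component.
; Its construction script applies the material at Index in a Material array to the sphere's first slot and swaps in a configurable mesh, NewMesh.
; It also stores the chosen material in ActiveMat.
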(fn ConstructionScript
  (Rendering|Material|SetMaterial (Variables|Default|GetSphere) 0 (Utilities|Array|Get(acopy) (Variables|Default|GetMaterial) (Variables|Default|GetIndex)))
  (Components|StaticMesh|SetStaticMesh (Variables|Default|GetSphere) (Variables|Default|GetNew%20Mesh))
  (Variables|Default|SetActive%20Mat (Utilities|Array|Get(acopy) (Variables|Default|GetMaterial) (Variables|Default|GetIndex))))