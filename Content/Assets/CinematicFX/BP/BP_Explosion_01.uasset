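; BP_Explosion_01 is a cinematic explosion effect actor built from core explosion, shockwave, sparks-and-debris and smoke Niagara components.
; The construction script assigns core and shockwave systems, enables auto-activation and passes a shared Scaler to all four.
; Six seconds after BeginPlay, it destroys itself unless Loop is set.
; When looping, a timeline's Update feeds a five-second Delay that reactivates all four effects with reset.
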(event EventBeginPlay
  (Utilities|FlowControl|Delay 6.0)
  (if (Variables|Default|GetLoop)
    (Timeline|Timeline_Explosion Play
      (:Update
        (Utilities|FlowControl|Delay 5.0)
        (Components|Activation|Activate (Variables|Default|GetCoreExplosion) true)))
    (else
      (Actor|DestroyActor))))

(event Collision|EventActorBeginOverlap
  (params (OtherActor :type Actor%20Object%20Reference)))

(event EventTick
  (params (DeltaSeconds :type Float%20%28single-precision%29)))

(fn ConstructionScript
  (Class|NiagaraComponent|SetAsset (Variables|Default|GetCoreExplosion) (Variables|Default|GetNS_Explosion) true)
  (Class|NiagaraComponent|SetAsset (Variables|Default|GetShockwave) (Variables|Default|GetNS_Shockwave) true)
  (Components|Activation|SetAutoActivate (Variables|Default|GetShockwave) true)
  (Niagara|SetNiagaraVariable(Float) (Variables|Default|GetCoreExplosion) "Scaler" (Variables|Default|GetScaler)))