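; BP_Shooting is a cinematic FX actor that automatically fires BP_Projectile toward a scattered target area.
; On BeginPlay, a Timeline's updates feed a one-second Delay that paces visibility line traces from the actor toward a far world point derived from Direction.
; Each hit spawns a projectile at the actor, adding physics velocity at random speed toward a random point in a flat horizontal box around the impact.
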(event EventBeginPlay
  (bind _returnvalue (Transformation|GetActorLocation))
  (Timeline|Timeline_0 Play
    (:Update
      (Utilities|FlowControl|Delay 1.0)
      (bind (_outhit _returnvalue_2) (Collision|LineTraceByChannel (Transformation|GetActorLocation) (* (Math|Vector|Normalize (Variables|Default|GetDirection)) 1e+09) "TraceTypeQuery1" false 0 "None"))
      (if _returnvalue_2
        (bind _output_get (Variables|Default|SetTraceLocation (.ImpactPoint (Collision|BreakHitResult _outhit))))
        (bind _returnvalue_3 (Game|SpawnActorfromClass "/Game/Assets/CinematicFX/BP/BP_Projectile.BP_Projectile_C" (Math|Transform|MakeTransform _returnvalue "0, 0, 0" "1.000000,1.000000,1.000000") "Undefined" "OverrideRootScale" 0 0))
        (Physics|SetPhysicsLinearVelocity (Variables|/Game/Assets/CinematicFX/BP/BP_Projectile.BP_Projectile_C|GetCollision _returnvalue_3) (* (Math|Vector|Normalize (- (Math|Random|RandomPointinBoundingBox _output_get "1000.000000,1000.000000, 0") _returnvalue)) (Math|Random|RandomFloatinRange 4e+03 8e+03)) true "None")))))

(event Collision|EventActorBeginOverlap
  (params (OtherActor :type Actor%20Object%20Reference)))

(event EventTick
  (params (DeltaSeconds :type Float%20%28single-precision%29)))

(fn ConstructionScript)