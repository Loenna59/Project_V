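; BP_Projectile is a cinematic FX projectile that explodes when its collision component hits something.
; On hit it plays a distance-based world camera shake and spawns a random actor from the Explosions array at the Projectile component's location.
; It then deactivates the FX, stops physics, hides its components and destroys itself after a short delay.
; The construction script hides the Projectile component and passes Scaler to the FX.
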(event OnComponentHit(Collision)
  (params (HitComponent :type Primitive%20Component%20Object%20Reference) (OtherActor :type Actor%20Object%20Reference) (OtherComp :type Primitive%20Component%20Object%20Reference) (NormalImpulse :type Vector :default "0, 0, 0") (Hit :type Hit%20Result%20Structure%20%28by%20ref%29))
  (bind _explosions (Variables|Default|GetExplosions))
  (bind _collision (Variables|Default|GetCollision))
  (Camera|PlayWorldCameraShake "/Game/Assets/CinematicFX/BP/BP_CameraShake.BP_CameraShake_C" (Transformation|GetActorLocation) 2e+02 5e+03)
  (Game|SpawnActorfromClass (Utilities|Array|Get(acopy) _explosions (Math|Random|RandomIntegerinRange 0 (- (Utilities|Array|Length _explosions) 1))) (Math|Transform|MakeTransform (Transformation|GetWorldLocation (Variables|Default|GetProjectile)) "0, 0, 0" "1.000000,1.000000,1.000000") "Undefined" "SelectDefaultAtRuntime" 0 0)
  (Components|Activation|Deactivate (Variables|Default|GetFX))
  (Physics|SetSimulatePhysics _collision false)
  (Rendering|SetVisibility _collision false false)
  (Utilities|FlowControl|Delay 2.0)
  (Actor|DestroyActor))

(fn ConstructionScript
  (Rendering|SetVisibility (Variables|Default|GetProjectile) false false)
  (Niagara|SetNiagaraVariable(Float) (Variables|Default|GetFX) "Scaler" (Variables|Default|GetScaler)))