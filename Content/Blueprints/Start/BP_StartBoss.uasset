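; BP_StartBoss is an actor that shows a sci-fi beast running continuously along a spline path.
; BeginPlay starts a looping run animation on the skeletal mesh.
; Tick advances a distance by Speed and delta time, then moves the mesh to that point in spline local space, with a yaw offset to align it with the path.
; The distance resets to zero past the spline's end, so the run repeats.
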(event EventBeginPlay
  (Components|Animation|PlayAnimation (Variables|Default|GetSkeletalMesh) "/Game/Assets/SciFi_Beasts_Pack/SciFi_Beast05/Animations/Anim_SciFi_Beast05_run1.Anim_SciFi_Beast05_run1" true))

(event Collision|EventActorBeginOverlap
  (params (OtherActor :type Actor%20Object%20Reference)))

(event EventTick
  (params (DeltaSeconds :type Float%20%28single-precision%29))
  (Variables|Default|Setdist (+ (* DeltaSeconds (Variables|Default|Getspeed)) (Variables|Default|Getdist)))
  (Transformation|SetRelativeTransform (Variables|Default|GetSkeletalMesh) (Math|Transform|MakeTransform (.location (Spline|GetTransformatDistanceAlongSpline (Variables|Default|GetSpline) (Variables|Default|Getdist) "Local" false)) (Math|Rotator|MakeRotator (.roll (.rotation (Spline|GetTransformatDistanceAlongSpline (Variables|Default|GetSpline) (Variables|Default|Getdist) "Local" false))) (.pitch (.rotation (Spline|GetTransformatDistanceAlongSpline (Variables|Default|GetSpline) (Variables|Default|Getdist) "Local" false))) (+ (.yaw (.rotation (Spline|GetTransformatDistanceAlongSpline (Variables|Default|GetSpline) (Variables|Default|Getdist) "Local" false))) -9e+01)) (Variables|/Script/Engine.SceneComponent|GetRelativeScale3D (Variables|Default|GetSkeletalMesh))) false false)
  (if (> (Variables|Default|Getdist) (Spline|GetSplineLength (Variables|Default|GetSpline)))
    (Variables|Default|Setdist 0.0)))

(fn ConstructionScript)